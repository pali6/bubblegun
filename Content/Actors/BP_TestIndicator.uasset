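; BP_TestIndicator is an actor that gives visual and audio feedback when an observed test succeeds.
; On BeginPlay it creates a dynamic material instance on its Sphere and binds to the ObservedTest's OnSucceed event.
; When that event fires, it sets the material's Tint parameter to green and plays SuccessSound at the actor's location.
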(event `self.ReceiveBeginPlay`
  (bind _sphere (`self.Sphere`))
  (bind _returnvalue (`PrimitiveComponent.CreateDynamicMaterialInstance` _sphere 0 (`PrimitiveComponent.GetMaterial` _sphere 0) "None"))
  (set `self.Material` _returnvalue)
  (add `/Game/Actors/A_BubbleTest.OnSucceed` (`self.ObservedTest`) (delegate `OnSucceed_Event`)))

(event `OnSucceed_Event`
  (`MaterialInstanceDynamic.SetVectorParameterValue` (`self.Material`) "Tint" (struct :`R` 0.069075 :`G` 1.0 :`A` 1.0))
  (`GameplayStatics.PlaySoundAtLocation` (`self.SuccessSound`) (`self.K2_GetActorLocation`) (struct) 1.0 1.0 0.0 null null null null))

(fn `UserConstructionScript`)