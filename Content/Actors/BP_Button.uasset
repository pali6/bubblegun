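; BP_Button is an interactable button actor that notifies listeners when pressed and animates its press.
; Interact passes through a DoOnce gate that resets after a half-second delay, so repeated presses are throttled.
; Each press calls the OnPressed dispatcher and plays the ButtonPress timeline, which lerps the button mesh's local Z down from its BeginPlay height by ButtonPressedDisplacement.
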(event `self.ReceiveBeginPlay`
  (set `self.ButtonBaseHeight` (.z (`SceneComponent.RelativeLocation` (`self.Button`)))))

(event `/Game/Blueprints/BI_Interactable.Interact`
  (bind _buttonbaseheight (`self.ButtonBaseHeight`))
  (bind _button (`self.Button`))
  (`/Engine/EditorBlueprintResources/StandardMacros.DoOnce` false :!label _label
    (:`Completed`
      (`|ExecutionSequence`
        (:`then_0`
          (`KismetSystemLibrary.Delay` 0.5)
          (goto _label :!via `Reset`))
        (:`then_1`
          (`self.OnPressed`)
          (bind (_direction _buttonheight) (`Timeline|Button Press` :!via `PlayFromStart`)
            (:`Update`
              (`SceneComponent.K2_SetRelativeLocation` _button (`KismetMathLibrary.MakeVector` (.x (`SceneComponent.RelativeLocation` _button)) (.y (`SceneComponent.RelativeLocation` _button)) (`KismetMathLibrary.Lerp` _buttonbaseheight (- _buttonbaseheight (`self.ButtonPressedDisplacement`)) _buttonheight)) false false))))))))

(fn `UserConstructionScript`)