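; BP_TestDoor is a door actor that moves from its start location by a target offset while all its linked tests report success.
; Every Tick it ANDs the IsSuccessful flag of each entry in Tests, so an empty list also counts as success.
; While that holds, a countdown timer drives a linear location lerp over Duration, without sweep.
; If a test stops succeeding, the door pauses in place rather than returning.
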(event `self.ReceiveBeginPlay`
  (set `self.Original Location` (`self.K2_GetActorLocation`))
  (set `self.Timer` (`self.Duration`)))

(event `self.ReceiveTick`
  (params (DeltaSeconds :type "Float (single-precision)"))
  (bind _original_location (`self.Original Location`))
  (`|ExecutionSequence`
    (:`then_0`
      (set `self.ShouldMove` true)
      (for _array_element (`self.Tests`)
        (set `self.ShouldMove` (and (`self.ShouldMove`) (`/Game/Actors/A_BubbleTest.IsSuccessful` _array_element)))))
    (:`then_1`
      (if (`self.ShouldMove`)
        (set `self.Timer` (- (`self.Timer`) DeltaSeconds))
        (`self.K2_SetActorLocation` (`KismetMathLibrary.VLerp` _original_location (+ _original_location (`self.TargetOffset`)) (- 1.0 (`KismetMathLibrary.FClamp` (/ (`self.Timer`) (`self.Duration`))))))))))

(fn `UserConstructionScript`)