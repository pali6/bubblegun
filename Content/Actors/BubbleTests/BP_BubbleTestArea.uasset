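; Bubble test area actor that detects when a Bubble reaches a target area.
; Each Tick, until success, it measures the distance from the TargetArea location to the Bubble's location offset by its CenterOfMass.
; When that distance falls below TargetRange, it sets IsSuccessful and fires the OnSucceed dispatcher once.
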(event `self.ReceiveBeginPlay`
  (`parent.ReceiveBeginPlay`))

(event `self.ReceiveTick`
  (params (DeltaSeconds :type "Float (single-precision)"))
  (bind _bubble (`self.Bubble`))
  (`parent.ReceiveTick` DeltaSeconds)
  (if (`self.IsSuccessful`)
    _
    (elif (< (`KismetMathLibrary.Vector_Distance` (`self.K2_GetActorLocation` (`self.TargetArea`)) (+ (`self.K2_GetActorLocation` _bubble) (`Bubble.CenterOfMass` _bubble))) (`self.TargetRange`))
      (set `self.IsSuccessful` true)
      (`self.OnSucceed`))))

(fn `UserConstructionScript`
  (`parent.UserConstructionScript`))