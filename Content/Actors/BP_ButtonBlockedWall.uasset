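; BP_ButtonBlockedWall is a wall that opens when its two buttons are pressed within a short time window of each other, in either order.
; Each button press starts or restarts that button's own timer, lasting ResetDuration, which invalidates its handle on expiry.
; A press while the other button's timer handle is still valid calls Open, which destroys the actor.
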(event `self.Button1.OnPressed`
  (if (`KismetSystemLibrary.K2_IsValidTimerHandle` (`self.Button2TImer`))
    (`self.Open`)
    (else
      (`KismetSystemLibrary.K2_ClearAndInvalidateTimerHandle` (`self.Button1Timer`))
      (bind _returnvalue (`KismetSystemLibrary.K2_SetTimerDelegate` (delegate `CustomEvent`) (`self.ResetDuration`)))
      (set `self.Button1Timer` _returnvalue))))

(event `CustomEvent`
  (`KismetSystemLibrary.K2_ClearAndInvalidateTimerHandle` (`self.Button1Timer`)))

(event `self.Button2.OnPressed`
  (if (`KismetSystemLibrary.K2_IsValidTimerHandle` (`self.Button1Timer`))
    (`self.Open`)
    (else
      (`KismetSystemLibrary.K2_ClearAndInvalidateTimerHandle` (`self.Button2TImer`))
      (bind _returnvalue (`KismetSystemLibrary.K2_SetTimerDelegate` (delegate `CustomEvent_1`) (`self.ResetDuration`)))
      (set `self.Button2TImer` _returnvalue))))

(event `CustomEvent_1`
  (`KismetSystemLibrary.K2_ClearAndInvalidateTimerHandle` (`self.Button2TImer`)))

(event `Open`
  (`self.K2_DestroyActor`))

(fn `UserConstructionScript`)