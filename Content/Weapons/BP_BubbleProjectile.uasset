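; Bubble projectile Blueprint that gives each spawned bubble a random color and delays its blocking of pawns.
; On BeginPlay, it creates a dynamic material instance on the mesh and sets BaseColor from a random, fully saturated HSV hue.
; After a short delay, it switches the collision component's Pawn channel response to Block.
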(event `self.ReceiveBeginPlay`
  ; Random Color on Spawn
  (bind _returnvalue (`PrimitiveComponent.CreateDynamicMaterialInstance` (`self.StaticMesh`) 0 (`PrimitiveComponent.GetMaterial` (`self.StaticMesh`) 0) "None"))
  (`MaterialInstanceDynamic.SetVectorParameterValue` _returnvalue "BaseColor" (`KismetMathLibrary.HSVToRGBLinear` (make `LinearColor` (* (`KismetMathLibrary.RandomFloat`) 360.0) 1.0 1.0 1.0)))
  (`KismetSystemLibrary.Delay` 0.3)
  (`PrimitiveComponent.SetCollisionResponseToChannel` (`self.CollisionComp`) "ECC_Pawn" "ECR_Block"))

(fn `UserConstructionScript`)