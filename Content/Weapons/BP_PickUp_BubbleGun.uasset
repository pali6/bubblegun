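; Pickup actor that gives the character a bubble gun when its TP_PickUp component fires OnPickUp.
; It adds a BPBubbleGun component to that character at runtime, attaches it at the GripPoint socket and stores it as WeaponComp.
; It then sets HasRifle on the first-person mesh's bubble gun AnimBP, invokes CallOnPickup and destroys itself.
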(event `self.TP_PickUp.OnPickUp`
  (params (PickUpCharacter :type "BubblegunCharacter Object Reference"))
  (bind _returnvalue (`|AddComponentByClass` :`self` PickUpCharacter :`Class` (`GameplayStatics.GetObjectClass` (`self.BP_BubbleGun`))))
  (`BubblegunWeaponComponent.AttachWeapon` _returnvalue PickUpCharacter "GripPoint")
  (set `BubblegunCharacter.WeaponComp` _returnvalue PickUpCharacter)
  (bind _asabp_first_person_bubble_gun (cast `/Game/PlayerCharacter/Animations/ABP_FirstPerson_BubbleGun` (`SkeletalMeshComponent.GetAnimInstance` (`BubblegunCharacter.Mesh1P` PickUpCharacter)))
    (:`then`
      (set `/Game/PlayerCharacter/Animations/ABP_FirstPerson_BubbleGun.HasRifle` true _asabp_first_person_bubble_gun))
    (:`CastFailed`
      _))
  (`self.On Pickup`)
  (`self.K2_DestroyActor`))

(fn `UserConstructionScript`)